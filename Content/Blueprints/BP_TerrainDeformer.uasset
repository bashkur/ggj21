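; Deformable ground actor that records digs in a render target, which feeds its landscape deform material as a displacement texture.
; Construction creates dynamic ground and dig-brush materials, and BeginPlay creates a white-cleared 8K render target and binds it to the ground.
; GroundHit draws the brush into that target at the hit UV, scaled by DigScale and rotated by the supplied angle, so marks accumulate.
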(event Custom|GroundHit
  (params (UVLocation :type Vector%202D%20Structure) (Rotation :type Float%20%28single-precision%29))
  (bind (_canvas _size _context) (Rendering|BeginDrawCanvastoRenderTarget (Variables|Default|GetLand)))
  (Canvas|DrawMaterial :self _canvas :RenderMaterial (Variables|Default|GetImpact) :ScreenPosition (.Screen%20Position (CallFunction|SetCanvasMaterialScaleandPosition _size UVLocation (Variables|Default|GetDigScale))) :ScreenSize (.Screen%20Size (CallFunction|SetCanvasMaterialScaleandPosition _size UVLocation (Variables|Default|GetDigScale))) :CoordinateSize "(X=1.000000,Y=1.000000)" :Rotation (+ (* Rotation -1.0) -9e+01) :PivotPoint "(X=0.500000,Y=0.500000)")
  (Rendering|EndDrawCanvastoRenderTarget _context))

(event EventBeginPlay
  (CallFunction|RenderTarget))

(event Collision|EventActorBeginOverlap
  (params (OtherActor :type Actor%20Object%20Reference)))

(event EventTick
  (params (DeltaSeconds :type Float%20%28single-precision%29)))

(fn ConstructionScript
  (bind _returnvalue (Rendering|Material|CreateDynamicMaterialInstance (Variables|Debug|GetStaticMeshComponent) 0 "/Game/Materials/M_LandscapeDeform.M_LandscapeDeform" "None" :!class /Script/Engine.PrimitiveComponent))
  (Variables|Default|SetGround _returnvalue)
  (bind _returnvalue_2 (Rendering|Material|CreateDynamicMaterialInstance "/Game/Materials/M_Dig.M_Dig" "None" :!class /Script/Engine.KismetMaterialLibrary))
  (bind _output_get (Variables|Default|SetImpact _returnvalue_2))
  (Rendering|Material|SetScalarParameterValue _output_get "Strength" (Variables|Default|GetDigStrength) :!class /Script/Engine.MaterialInstanceDynamic)
  (Rendering|Material|SetScalarParameterValue (Variables|Default|GetImpact) "UpMultiplier" (Variables|Default|GetUpMultiplier) :!class /Script/Engine.MaterialInstanceDynamic))

(fn RenderTarget
  (bind _returnvalue (Rendering|CreateRenderTarget2D 8192 8192 "RTF_RGBA8"))
  (bind _output_get (Variables|Default|SetLand _returnvalue))
  (Rendering|ClearRenderTarget2D _output_get "(R=1.000000,G=1.000000,B=1.000000,A=1.000000)")
  (Rendering|Material|SetTextureParameterValue (Variables|Default|GetGround) "Displacement" _output_get))