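; BP_ShovelTool is a digging tool whose Dig event marks deformable terrain where its owner is looking.
; It line-traces a short distance forward from the owner's camera against complex Visibility collision, with debug drawing left on.
; When the hit actor is a BP_TerrainDeformer, it finds the collision UV on channel 1 and passes it to GroundHit with the owner's skeletal mesh yaw.
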(event EventDig
  (bind _returnvalue (Components|GetOwner))
  (bind _returnvalue_2 (Actor|GetComponentbyClass _returnvalue "/Script/Engine.CameraComponent"))
  (bind _returnvalue_3 (Transformation|GetWorldLocation _returnvalue_2))
  (bind (_outhit _returnvalue_4) (Collision|LineTraceByChannel _returnvalue_3 (+ _returnvalue_3 (* (Math|Vector|GetForwardVector _returnvalue_2) 3e+02)) "TraceTypeQuery1" true 0 "ForDuration"))
  (if _returnvalue_4
    (bind _asbp_terrain_deformer (Utilities|Casting|CastToBP_TerrainDeformer (.HitActor (Collision|BreakHitResult _outhit))))
    (Default|GroundHit _asbp_terrain_deformer (.UV (Class|GameplayStatics|FindCollisionUV _outhit 1)) (.yaw (Transformation|GetWorldRotation (Actor|GetComponentbyClass _returnvalue "/Script/Engine.SkeletalMeshComponent"))))))