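; BP_TreasureSpawner is a work-in-progress treasure placement Blueprint that currently only tests a random spawn point and spawns nothing.
; On BeginPlay it queries the NavMesh for a reachable point within SpawnRadius of its owner's location.
; A box trace at that point checks that the hit actor's sole tag is "Ground", with debug shapes and prints showing results.
; The loop over the Treasures array is disconnected and never runs.
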(event EventBeginPlay
  (bind _output_get (Variables|Default|SetSelfPos (Transformation|GetActorLocation (Components|GetOwner self))))
  (Rendering|Debug|DrawDebugSphere _output_get (Variables|Default|GetSpawnRadius) 12 "(R=0.000000,G=1.000000,B=0.078335,A=1.000000)" 1e+02)
  (bind _output_get_2 (Variables|Default|SetTempRandomPos (.RandomLocation (AI|Navigation|GetRandomReachablePointinRadius (Variables|Default|GetSelfPos) (Variables|Default|GetSpawnRadius) 0 0))))
  (if (.ReturnValue (AI|Navigation|GetRandomReachablePointinRadius (Variables|Default|GetSelfPos) (Variables|Default|GetSpawnRadius) 0 0))
    (Rendering|Debug|DrawDebugSphere _output_get_2 1e+02 12 "(R=0.000000,G=0.882243,B=1.000000,A=1.000000)" 1e+01)
    (Development|PrintString (Utilities|String|ToString(Vector) _output_get_2) true true "(R=0.000000,G=0.060000,B=0.992000,A=1.000000)" 5.0)
    (bind _outhit (Collision|BoxTraceByChannel _output_get_2 (+ _output_get_2 "0, 0,-1.000000") "100.000000,100.000000,10.000000" "0,1.000000, 0" "TraceTypeQuery1" false 0 "ForDuration"))
    (if (and (Utilities|Array|ContainsItem (Variables|/Script/Engine.Actor|GetTags (.HitActor (Collision|BreakHitResult _outhit))) "Ground") (== (Utilities|Array|Length (Variables|/Script/Engine.Actor|GetTags (.HitActor (Collision|BreakHitResult _outhit)))) 1))
      (Development|PrintString "Good" true true "(R=0.000000,G=0.660000,B=1.000000,A=1.000000)" 5.0))
    (else
      (Development|PrintString "NavMesh couldn't find point" true true "(R=1.000000,G=0.000000,B=0.000000,A=1.000000)" 5.0))))

(event Collision|EventActorBeginOverlap
  (params (OtherActor :type Actor%20Object%20Reference)))

(event EventTick
  (params (DeltaSeconds :type Float%20%28single-precision%29)))

(fn ConstructionScript)