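; BP_Treasure is a treasure actor with a configurable mesh and functions for being found and collected.
; Found prints a message and snaps the actor onto the navmesh; Collect teleports it to the CollectionPosition actor.
; The construction script applies the mesh and uses a self-resetting Test boolean to trigger Found in the editor.
; Detection radius setup and the Collect test call are disconnected, and the event graph is empty.
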(event EventBeginPlay)

(event Collision|EventActorBeginOverlap
  (params (OtherActor :type Actor%20Object%20Reference)))

(event EventTick
  (params (DeltaSeconds :type Float%20%28single-precision%29)))

(fn ConstructionScript
  (Components|StaticMesh|SetStaticMesh (Variables|Default|GetStaticMesh) (Variables|Default|GetTreasureMesh))
  (if (Variables|Default|Gettest)
    (CallFunction|Found)
    (Variables|Default|Settest false)))

(fn Found
  (bind _self self)
  (bind _returnvalue (Transformation|GetActorLocation _self))
  (bind _projectedlocation (AI|Navigation|ProjectPointtoNavigation _returnvalue 0 0 "0, 0, 0"))
  (Development|PrintString "Found")
  (Transformation|SetActorLocation _projectedlocation false true)
  (Transformation|SetActorLocation _projectedlocation false true))

(fn Collect
  (Transformation|SetActorLocation (Transformation|GetActorLocation (Variables|Default|GetCollectionPosition)) false true))