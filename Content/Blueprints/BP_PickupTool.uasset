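; BP_PickupTool is a tool on GGJ21Character that lets the player pick up BP_Treasure actors they look at.
; BeginPlay creates a hidden WBP_Pickup widget and caches the owning character.
; Tick traces a short line from the owner's camera, showing the prompt only over treasure while ActiveTool is 1.
; The Pickup event repeats the trace with complex collision and destroys the treasure hit, without checking the active tool.
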(event EventBeginPlay
  (bind _returnvalue (UserInterface|CreateWidget "/Game/UI/WBP_Pickup.WBP_Pickup_C" (Game|GetPlayerController 0)))
  (bind _output_get (Variables|Default|Setpickup_widget _returnvalue))
  (UserInterface|Viewport|AddtoViewport _output_get 0)
  (Widget|SetVisibility _output_get "Hidden")
  (bind _asggj21character (Utilities|Casting|CastToGGJ21Character (Components|GetOwner)))
  (Variables|Default|Setchar _asggj21character))

(event EventPickup
  (bind _returnvalue (Components|GetOwner))
  (bind _returnvalue_2 (Actor|GetComponentbyClass _returnvalue "/Script/Engine.CameraComponent"))
  (bind _returnvalue_3 (Transformation|GetWorldLocation _returnvalue_2))
  (bind (_outhit _returnvalue_4) (Collision|LineTraceByChannel _returnvalue_3 (+ _returnvalue_3 (* (Math|Vector|GetForwardVector _returnvalue_2) 3e+02)) "TraceTypeQuery1" true 0 "None"))
  (if _returnvalue_4
    (bind _asbp_treasure (Utilities|Casting|CastToBP_Treasure (.HitActor (Collision|BreakHitResult _outhit))))
    (Actor|DestroyActor _asbp_treasure)))

(event EventTick
  (params (DeltaSeconds :type Float%20%28single-precision%29))
  (bind _returnvalue (Components|GetOwner))
  (bind _pickup_widget (Variables|Default|Getpickup_widget))
  (bind _returnvalue_2 (Actor|GetComponentbyClass _returnvalue "/Script/Engine.CameraComponent"))
  (bind _returnvalue_3 (Transformation|GetWorldLocation _returnvalue_2))
  (bind (_outhit _returnvalue_4) (Collision|LineTraceByChannel _returnvalue_3 (+ _returnvalue_3 (* (Math|Vector|GetForwardVector _returnvalue_2) 3e+02)) "TraceTypeQuery1" false 0 "None"))
  (if _returnvalue_4
    (Utilities|Casting|CastToBP_Treasure (.HitActor (Collision|BreakHitResult _outhit))
      (:then
        (if (== (Variables|/Script/GGJ21.GGJ21Character|GetActiveTool (Variables|Default|Getchar)) 1)
          (Widget|SetVisibility _pickup_widget "Visible")
          (else
            (Widget|SetVisibility _pickup_widget "Hidden" :!label _label))))
      (:CastFailed
        (goto _label)))
    (else
      (goto _label))))