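; BP_MapTool lets the player bring out and put away a map in the game.
; ToggleMap finds the player character's scene component tagged "Map" and flips the MapOn state.
; When on, it spawns a map actor at that component's transform with a yaw offset and attaches it to the pawn's root, keeping world transform.
; When off, it destroys the stored map actor.
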(event EventBeginPlay)

(event EventTick
  (params (DeltaSeconds :type Float%20%28single-precision%29)))

(event EventToggleMap
  (bind _returnvalue (Game|Player|GetPlayerPawn 0))
  (bind _asggj21character (Utilities|Casting|CastToGGJ21Character _returnvalue))
  (bind _asscene_component (Utilities|Casting|CastToSceneComponent (Utilities|Array|Get(acopy) (Actor|GetComponentsbyTag _asggj21character "/Script/Engine.SceneComponent" "Map"))))
  (bind _output_get (Variables|Default|SetMapOn (not (Variables|Default|GetMapOn))))
  (if _output_get
    (bind _returnvalue_2 (Game|SpawnActorfromClass "/Game/Developers/Zach/BP_Map.BP_Map_C" (Math|Transform|MakeTransform (.location (Transformation|GetWorldTransform _asscene_component)) (Math|Rotator|MakeRotator (.Roll (Math|Rotator|BreakRotator (.rotation (Transformation|GetWorldTransform _asscene_component)))) (.Pitch (Math|Rotator|BreakRotator (.rotation (Transformation|GetWorldTransform _asscene_component)))) (+ (.Yaw (Math|Rotator|BreakRotator (.rotation (Transformation|GetWorldTransform _asscene_component)))) 9e+01)) (.scale (Transformation|GetWorldTransform _asscene_component))) "AlwaysSpawn" 0 0))
    (bind _output_get_2 (Variables|Default|SetMapRef _returnvalue_2))
    (Transformation|AttachComponentToComponent _output_get_2 (Variables|/Script/Engine.Actor|GetRootComponent _returnvalue) "None" "KeepWorld" "KeepWorld" "KeepWorld" false)
    (else
      (Actor|DestroyActor (Variables|Default|GetMapRef)))))